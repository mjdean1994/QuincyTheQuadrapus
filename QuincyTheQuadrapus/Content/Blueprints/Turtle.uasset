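; Turtle actor that moves in a continuous loop through an array of waypoint actors.
; Each Tick, HandleMovement advances the target index on coming within a small distance of the current waypoint, wrapping to the first after the last.
; It turns the Scene component toward the target and steps the actor along the normalized direction at MoveSpeed scaled by delta time, without sweeping for collision.
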(event EventBeginPlay)

(event Collision|EventActorBeginOverlap
  (params (OtherActor :type Actor%20Object%20Reference)))

(event EventTick
  (params (DeltaSeconds :type Float%20%28single-precision%29))
  (CallFunction|HandleMovement DeltaSeconds))

(fn ConstructionScript)

(fn HandleMovement
  (params (Delta :type Float%20%28single-precision%29))
  (LocalVariables|SetCurrent (Transformation|GetActorLocation))
  (LocalVariables|SetTarget (Transformation|GetActorLocation (Utilities|Array|Get(acopy) (Variables|Default|GetWaypoints) (Variables|Default|GetCurrentTargetIndex))))
  (if (Math|Vector|Equal(Vector) (LocalVariables|GetCurrent) (LocalVariables|GetTarget) 1e+01)
    (bind _result (Math|Integer|IncrementInt (Variables|Default|GetCurrentTargetIndex))
      (:%20%20
        (if (> _result (- (Utilities|Array|Length (Variables|Default|GetWaypoints)) 1))
          (Variables|Default|SetCurrentTargetIndex 0)
          (LocalVariables|SetTarget (Transformation|GetActorLocation (Utilities|Array|Get(acopy) (Variables|Default|GetWaypoints) (Variables|Default|GetCurrentTargetIndex))) :!label _label)
          (Transformation|SetWorldRotation (Variables|Default|GetScene) (Math|Rotator|FindLookatRotation (LocalVariables|GetCurrent) (LocalVariables|GetTarget)) false false)
          (Transformation|SetActorLocation (+ (LocalVariables|GetCurrent) (* (Math|Vector|Normalize (- (LocalVariables|GetTarget) (LocalVariables|GetCurrent))) (* Delta (Variables|Default|GetMoveSpeed)))) false false))))
    (else
      (goto _label))))