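; Time utility with a FloatToTime function that converts a float in seconds into a minutes:seconds.hundredths display string.
; It derives minutes and leftover seconds by truncation, then formats each part with digit limits and zero-padding before appending.
; The value named Milliseconds is in hundredths and subtracts only the leftover seconds, so past one minute it relies on the two-digit limit to drop the excess.
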(fn FloattoTime
  (params (TimeIn :type Float%20%28single-precision%29))
  (bind _output_get (LocalVariables|SetMInutes (Math|Float|Truncate (/ TimeIn 6e+01))))
  (bind _output_get_2 (LocalVariables|SetSeconds (Math|Float|Truncate (- TimeIn (* _output_get 6e+01)))))
  (LocalVariables|SetMilliseconds (Math|Float|Truncate (* (- TimeIn (Math|Conversions|ToFloat(Integer) _output_get_2)) 1e+02)))
  (return (Utilities|String|Append (Utilities|String|Append (Utilities|String|Append (Utilities|String|ToString(Text) (Utilities|Text|ToText(Integer) (LocalVariables|GetMInutes) false true 1 4)) ":") (Utilities|String|Append (Utilities|String|ToString(Text) (Utilities|Text|ToText(Integer) (LocalVariables|GetSeconds) false true 2 2)) ".")) (Utilities|String|ToString(Text) (Utilities|Text|ToText(Integer) (LocalVariables|GetMilliseconds) false true 2 2)))))