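; JellyfishGlow is an actor Blueprint that bobs vertically between two world heights; despite its name, it contains no glow logic.
; Tick offsets the actor along Z by MoveSpeed scaled by delta time, without sweep, in the direction set by GoingUp.
; GoingUp flips once the actor's Z passes MaxHeight or MinHeight, giving a constant-speed ping-pong motion.
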(event EventBeginPlay)

(event Collision|EventActorBeginOverlap
  (params (OtherActor :type Actor%20Object%20Reference)))

(event EventTick
  (params (DeltaSeconds :type Float%20%28single-precision%29))
  (if (Variables|Default|GetGoingUp)
    (Transformation|AddActorWorldOffset (Math|Vector|MakeVector 0.0 0.0 (* DeltaSeconds (Variables|Default|GetMoveSpeed))))
    (if (> (.Z (Math|Vector|BreakVector (Transformation|GetActorLocation))) (Variables|Default|GetMaxHeight))
      (Variables|Default|SetGoingUp false))
    (else
      (Transformation|AddActorWorldOffset (Math|Vector|MakeVector 0.0 0.0 (* (* DeltaSeconds -1.0) (Variables|Default|GetMoveSpeed))))
      (if (< (.Z (Math|Vector|BreakVector (Transformation|GetActorLocation))) (Variables|Default|GetMinHeight))
        (Variables|Default|SetGoingUp true)))))

(fn ConstructionScript)